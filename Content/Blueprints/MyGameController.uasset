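; Player controller that spawns purchasable items on a repeating timer and lets the player buy them with a mouse click.
; A delay loop drops a BP_Item at one of three random positions from the level's BP_SpawnItemPos actor.
; Clicks line-trace from the cursor, call Buy on the hit item and store it as selected.
; It also caches the camera pawn and one team's characters, whose charge UpdateChargingEat reduces.
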(event `self.ReceiveBeginPlay`
  (`|ExecutionSequence`
    (:`then_0`
      (`KismetSystemLibrary.Delay` 2.0)
      (`self.SpawnItems` :!label _label)
      (`KismetSystemLibrary.Delay` 3.0)
      (goto _label))
    (:`then_1`
      (set `self.bShowMouseCursor` true)
      (bind _asbp_camera (cast `/Game/Blueprints/BP_Camera` (`GameplayStatics.GetPlayerPawn` 0)))
      (set `self.As BP Camera` _asbp_camera)
      (`self.AddCharacterTeam`))))

(event `EnhancedInput|/Game/Input/I_Click`
  (params (ActionValue :type Boolean) (ElapsedSeconds :type "Float (double-precision)") (TriggeredSeconds :type "Float (double-precision)") (InputAction :type "InputAction Object Reference" :default "/Game/Input/I_Click.I_Click"))
  (bind (_worldlocation _worlddirection) (`self.DeprojectMousePositionToWorld` (`GameplayStatics.GetPlayerController` 0)))
  (:`Started`
    (bind _outhit (`KismetSystemLibrary.LineTraceSingle` :`Start` _worldlocation :`End` (+ _worldlocation (* _worlddirection 5000.0)) :`TraceChannel` "TraceTypeQuery1" :`DrawDebugType` "Persistent"))
    (bind _asbp_item (cast `/Game/Blueprints/Items/BP_Item` (`.HitActor` (`GameplayStatics.BreakHitResult` _outhit))))
    (`/Game/Blueprints/Items/BP_Item.Buy` _asbp_item)
    (set `self.ItemSelected` _asbp_item)))

(fn `AddCharacterTeam`
  (bind _outactors (`GameplayStatics.GetAllActorsOfClass` "/Game/Blueprints/BP_CharacterBase.BP_CharacterBase_C"))
  (for _array_element _outactors
    (if (`|EnumEquality` (`/Game/Blueprints/BP_CharacterBase.Team` _array_element) "NewEnumerator0")
      (`KismetArrayLibrary.Array_AddUnique` (`self.ListCharacter`) _array_element))))

(fn `SpawnItems`
  (bind _spawpos (`self.SpawPos`))
  (switch `int` (`KismetMathLibrary.RandomIntegerInRange` 0 2)
    (:`0`
      (`|SpawnActorFromClass` "/Game/Blueprints/Items/BP_Item.BP_Item_C" (`KismetMathLibrary.MakeTransform` (`SceneComponent.GetSocketLocation` (`/Game/Blueprints/BP_SpawnItemPos.pos1` _spawpos) "None")) "AdjustIfPossibleButAlwaysSpawn" "OverrideRootScale" (`GameplayStatics.GetPlayerController` 0) (2608.941064 0.0 0.0) null))
    (:`1`
      (`|SpawnActorFromClass` "/Game/Blueprints/Items/BP_Item.BP_Item_C" (`KismetMathLibrary.MakeTransform` (`SceneComponent.K2_GetComponentLocation` (`/Game/Blueprints/BP_SpawnItemPos.pos2` _spawpos))) "AdjustIfPossibleButAlwaysSpawn" "OverrideRootScale" (`GameplayStatics.GetPlayerController` 0) (2608.941064 0.0 0.0) null))
    (:`2`
      (`|SpawnActorFromClass` "/Game/Blueprints/Items/BP_Item.BP_Item_C" (`KismetMathLibrary.MakeTransform` (`SceneComponent.K2_GetComponentLocation` (`/Game/Blueprints/BP_SpawnItemPos.pos3` _spawpos))) "AdjustIfPossibleButAlwaysSpawn" "OverrideRootScale" (`GameplayStatics.GetPlayerController` 0) (2608.941064 0.0 0.0) null))))

(fn `UpdateChargingEat`
  (for _array_element (`self.ListCharacter`)
    (set `/Game/Blueprints/BP_CharacterBase.CurrentCharging` (- (`/Game/Blueprints/BP_CharacterBase.CurrentCharging` _array_element) 20.0) _array_element)))

(fn `UserConstructionScript`
  (bind _returnvalue (`GameplayStatics.GetActorOfClass` "/Game/Blueprints/BP_SpawnItemPos.BP_SpawnItemPos_C"))
  (set `self.SpawPos` _returnvalue))