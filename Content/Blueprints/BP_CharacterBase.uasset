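; Base character that auto-fires bursts of elemental balls, with its ball stock doubling as HP.
; A repeating timed loop fills a charge bar, sped up by starting Water balls; when full, a delayed loop spawns team-tagged BP_Bullets with random ball types, sized from the stock total.
; UpdateBall removes one ball of the element paired with the incoming type, otherwise two random ones; Eat replenishes existing types.
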(event `self.ReceiveBeginPlay`
  (`self.SetSkill`)
  (`self.InitCurrentChargingspeed`)
  ;[1 1 1] sạc đạn và check nếu đủ 100% sẽ bắn
  (`self.UpdateCharging` :!label _label)
  (`self.Shoot`)
  (`KismetSystemLibrary.Delay` 0.1)
  (goto _label))

(event `Shoot`
  ;[1 1 1] bắn ra các loại đạn
  (if (>= (`self.CurrentCharging`) (`.MaxCharging_32_C848E9E14E23FDAE58A3FB8C5E7FE81E` (break `/Game/Data/S_Character` (`self.Base`))))
    (`self.UpdateCurrentCharging` -100.0)
    (`self.ForLoopWithDelay` 0 (- (`self.BallShootInTime`) 1) (/ (`self.AttackSpeed`) (`self.TotalBallShoot`))
      (:`Loop Body`
        (`self.SpawnBullet`)))))

(fn `Damaged`
  (params (Ball :type "/Game/Data/S_Ball Structure") (Index :type Integer))
  (bind (_typename _quantity _icon) (break `/Game/Data/S_Ball` Ball))
  (bind _result (`/Engine/EditorBlueprintResources/StandardMacros.DecrementInt` _quantity)
    (:`  `
      (if (<= _result 0)
        (`KismetArrayLibrary.Array_Remove` (`self.Balls`) Index)
        (else
          (setmembers `/Game/Data/S_Ball` :`StructRef` (`|GetArrayItem` (`self.Balls`) Index) :`TypeName` _typename :`Quantity` _result :`Icon` _icon)
          (`self.UpdateTotalBallExits`))))))

(fn `Die`
  (`KismetSystemLibrary.PrintString` "Die")
  (`self.K2_DestroyActor`))

(fn `Eat`
  (params (NewParam :type "Map of /Game/Data/E_Ball Enum to /Game/Data/S_Ball Structure"))
  (bind _balls (`self.Balls`))
  (for (_array_element _array_index) _balls
    (bind (_typename _quantity _icon) (break `/Game/Data/S_Ball` _array_element))
    (bind (_value _returnvalue) (`BlueprintMapLibrary.Map_Find` NewParam _typename))
    (if _returnvalue
      (`KismetArrayLibrary.Array_Set` _balls _array_index (make `/Game/Data/S_Ball` _typename (+ _quantity (`.Quantity_7_3FBFA38C4FDBAC1EC929379C197F5DCD` (break `/Game/Data/S_Ball` _value))) _icon))
      (`self.UpdateTotalBallExits`))))

(fn `Get Random Ball`
  (returns (Value :type "/Game/Data/S_Ball Structure") (Index :type Integer))
  (bind _returnvalue (`KismetArrayLibrary.Array_Length` (`self.Balls`)))
  (bind _returnvalue_2 (`KismetMathLibrary.RandomIntegerInRange` 0 (- _returnvalue 1)))
  (if (> _returnvalue 0)
    (return (`|GetArrayItem` (`self.Balls`) _returnvalue_2) _returnvalue_2)))

(fn `InitCurrentChargingspeed`
  (bind ((`ChargingSpeed_31_8C7C6A4F49A0E5010B46BE9FFD1660AD` _chargingspeed) (`TotalBall_25_FBD4C43B44058692EC1D8793327E564D` _totalball)) (break `/Game/Data/S_Character` (`self.Base`)))
  (set `self.Current Charging Speed` _chargingspeed)
  (for _array_element _totalball
    (bind (_typename _quantity) (break `/Game/Data/S_Ball` _array_element))
    (if (`|EnumEquality` _typename "NewEnumerator1")
      (set `self.Current Charging Speed` (+ (`self.Current Charging Speed`) _quantity)))))

(fn `SetSkill`
  ;[1 1 1] Lấy thông tin skill
  (`/Game/Blueprints/BPC_CreateSkill.CreatSkillFinish` (`self.BPC_CreateSkill`) (`self.TotalBallShoot`))
  (for _array_element (`/Game/Blueprints/BPC_CreateSkill.Skills` (`self.BPC_CreateSkill`))
    (`KismetArrayLibrary.Array_Add` (`.TotalBall_25_FBD4C43B44058692EC1D8793327E564D` (break `/Game/Data/S_Character` (`self.Base`))) _array_element)
    (`KismetArrayLibrary.Array_Add` (`self.Balls`) _array_element))
  (`self.UpdateTotalBallExits`)
  (set `self.BallShootInTime` (`KismetMathLibrary.FTrunc` (* (`self.TotalBallShoot`) 0.1))))

(fn `SpawnBullet`
  ;[1 1 1] Spawn và bắn
  (bind _returnvalue (`|SpawnActorFromClass` "/Game/Blueprints/Bullet/BP_Bullet.BP_Bullet_C" (`KismetMathLibrary.MakeTransform` (+ (.location (`self.GetTransform`)) (0.0 0.0 50.0)) (.rotation (`self.GetTransform`)) (* (.scale (`self.GetTransform`)) 0.3)) "AlwaysSpawn" "OverrideRootScale" null null))
  (set `/Game/Blueprints/Bullet/BP_Bullet.Team` (`self.Team`) _returnvalue)
  (bind _value (`self.Get Random Ball`))
  (set `/Game/Blueprints/Bullet/BP_Bullet.BallBase` _value _returnvalue))

(fn `TakeDamage`
  (params (EBall :type "/Game/Data/E_Ball Enum" :default "NewEnumerator0"))
  (returns (ReturnValue :type Boolean) (Ball :type "/Game/Data/S_Ball Structure") (`Array Index` :type Integer))
  (bind _balls (`self.Balls`))
  (if (`KismetArrayLibrary.Array_IsEmpty` _balls)
    (`self.K2_DestroyActor`)
    (else
      ;[1 1 1] Kiểm tra có loại bóng khac chế không
      (for (_array_element _array_index) _balls
        (bind _returnvalue (`|EnumEquality` (`.TypeName_5_BF24237E4E76D00722C82F9C894F6550` (break `/Game/Data/S_Ball` _array_element)) EBall))
        (if _returnvalue
          (break)))
      (return _returnvalue _array_element _array_index))))

(fn `UpdateBall`
  (params (BallDamage :type "/Game/Data/S_Ball Structure"))
  (switch `/Game/Data/E_Ball` (`.TypeName_5_BF24237E4E76D00722C82F9C894F6550` (break `/Game/Data/S_Ball` BallDamage))
    (:`NewEnumerator0`
      (bind (_returnvalue _ball _array_index) (`self.TakeDamage` "NewEnumerator1"))
      (if _returnvalue
        (`self.Damaged` _ball _array_index)
        (else
          (bind (_value _index) (`self.Get Random Ball` :!label _label))
          (`self.Damaged` _value _index)
          (bind (_value_2 _index_2) (`self.Get Random Ball`))
          (`self.Damaged` _value_2 _index_2))))
    (:`NewEnumerator1`
      (bind (_returnvalue_2 _ball_2 _array_index_2) (`self.TakeDamage` "NewEnumerator2"))
      (if _returnvalue_2
        (`self.Damaged` _ball_2 _array_index_2)
        (else
          (goto _label))))
    (:`NewEnumerator2`
      (bind (_returnvalue_3 _ball_3 _array_index_3) (`self.TakeDamage` "NewEnumerator0"))
      (if _returnvalue_3
        (`self.Damaged` _ball_3 _array_index_3)
        (else
          (goto _label))))
    (:`NewEnumerator3`
      (bind (_returnvalue_4 _ball_4 _array_index_4) (`self.TakeDamage` "NewEnumerator4"))
      (if _returnvalue_4
        (`self.Damaged` _ball_4 _array_index_4)
        (else
          (goto _label))))
    (:`NewEnumerator4`
      (bind (_returnvalue_5 _ball_5 _array_index_5) (`self.TakeDamage` "NewEnumerator3"))
      (if _returnvalue_5
        (`self.Damaged` _ball_5 _array_index_5)
        (else
          (goto _label))))))

(fn `UpdateCharging`
  ;[1 1 1] hồi tốc độ sạc đạn theo giây
  (`self.UpdateCurrentCharging` (/ (`self.Current Charging Speed`) 10.0)))

(fn `UpdateCurrentCharging`
  (params (Val :type "Float (double-precision)"))
  (bind _output_get (set `self.CurrentCharging` (+ (`self.CurrentCharging`) Val)))
  (bind _aswbp_charging (cast `/Game/Blueprints/UI/WBP_Charging` (`WidgetComponent.GetWidget` (`self.WBP_Charging`))))
  (`/Game/Blueprints/UI/WBP_Charging.UpdatePercent` _aswbp_charging _output_get (`.MaxCharging_32_C848E9E14E23FDAE58A3FB8C5E7FE81E` (break `/Game/Data/S_Character` (`self.Base`)))))

(fn `UpdateTotalBallExits`
  (set `self.TotalBallShoot` 0)
  (for _array_element (`self.Balls`)
    (bind _output_get (set `self.TotalBallShoot` (+ (`self.TotalBallShoot`) (`.Quantity_7_3FBFA38C4FDBAC1EC929379C197F5DCD` (break `/Game/Data/S_Ball` _array_element)))))
    (bind _aswbp_charging (cast `/Game/Blueprints/UI/WBP_Charging` (`WidgetComponent.GetWidget` (`self.WBP_Charging`))))
    (`/Game/Blueprints/UI/WBP_Charging.UpdateHp` _aswbp_charging _output_get)))

(fn `UserConstructionScript`)