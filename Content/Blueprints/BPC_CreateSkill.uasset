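; Component that randomly generates a character's skill set as three elemental balls with quantities, along with a weighted random level of 1 to 3.
; CreatSkillFinish loads element rows from DB_Ball and builds a pool weighted toward Fire, Water and Wood, with rare Lightning or Darkness.
; Retry loops pick three distinct types, then further draws from the shrinking pool raise their quantities before they are added to Skills.
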(event `self.ReceiveBeginPlay`)

(fn `AddListBall`
  (params (TotalBall :type Integer))
  (bind _listball (`self.ListBall`))
  (`|ExecutionSequence`
    (:`then_0`
      (for _ (range (+ (`KismetMathLibrary.FTrunc` (* TotalBall 0.05)) 1))
        (if (>= (`KismetMathLibrary.RandomIntegerInRange` 0 100) 50)
          (`KismetArrayLibrary.Array_Add` _listball (`self.Darkness`))
          (else
            (`KismetArrayLibrary.Array_Add` _listball (`self.Lightning`))))))
    (:`then_1`
      (for _ (range (+ (`KismetMathLibrary.FTrunc` (* TotalBall 0.33)) 1))
        (`KismetArrayLibrary.Array_Add` (`self.ListBall`) (`self.Fire`))))
    (:`then_2`
      (for _ (range (+ (`KismetMathLibrary.FTrunc` (* TotalBall 0.33)) 1))
        (`KismetArrayLibrary.Array_Add` (`self.ListBall`) (`self.Water`))))
    (:`then_3`
      (for _ (range (+ (`KismetMathLibrary.FTrunc` (* TotalBall 0.33)) 1))
        (`KismetArrayLibrary.Array_Add` (`self.ListBall`) (`self.Wood`))))))

(fn `CreateBallForCharacter`
  (`KismetArrayLibrary.Array_Add` (`self.Skills`) (`self.Ball1`))
  (`KismetArrayLibrary.Array_Add` (`self.Skills`) (`self.Ball2`))
  (`KismetArrayLibrary.Array_Add` (`self.Skills`) (`self.Ball3`)))

(fn `CreatSkillFinish`
  (params (Level :type Integer))
  (`self.GetLevel`)
  (`self.InitBall`)
  (`self.AddListBall` (`self.TotalBallInit`))
  (`self.GetRandomBallInit`)
  (for _ (range 1 (+ (- 20 3) 1))
    (`self.GetRandomBall`))
  (`self.CreateBallForCharacter`))

(fn `GetLevel`
  (bind _returnvalue (`KismetMathLibrary.RandomFloatInRange` 0.0 100.0))
  (if (<= _returnvalue 70.0)
    (set `self.Level` 1)
    (elif (<= _returnvalue 95.0)
      (set `self.Level` 2)
      (else
        (set `self.Level` 3)))))

(fn `GetRandomBall`
  (bind (_typename _quantity) (break `/Game/Data/S_Ball` (`self.Ball3`)))
  (bind (_typename_2 _quantity_2) (break `/Game/Data/S_Ball` (`self.Ball1`)))
  (bind (_typename_3 _quantity_3) (break `/Game/Data/S_Ball` (`self.Ball2`)))
  (bind _output_get (set `self.RandomValue` (`KismetMathLibrary.RandomIntegerInRange` 0 (`KismetArrayLibrary.Array_Length` (`self.ListBall`))) :!label _label))
  (bind _typename_4 (break `/Game/Data/S_Ball` (`|GetArrayItem` (`self.ListBall`) _output_get)))
  (if (`|EnumEquality` _typename_4 _typename_2)
    (`/Engine/EditorBlueprintResources/StandardMacros.IncrementInt` _quantity_2
      (:`  `
        _))
    (elif (`|EnumEquality` _typename_4 _typename_3)
      (`/Engine/EditorBlueprintResources/StandardMacros.IncrementInt` _quantity_3
        (:`  `
          _))
      (elif (`|EnumEquality` _typename_4 _typename)
        (`/Engine/EditorBlueprintResources/StandardMacros.IncrementInt` _quantity
          (:`  `
            _))
        (else
          (goto _label)))))
  (`KismetArrayLibrary.Array_Remove` (`self.ListBall`) (`self.RandomValue`)))

(fn `GetRandomBallInit`
  (bind _listball (`self.ListBall`))
  (bind _returnvalue (`KismetMathLibrary.RandomIntegerInRange` 0 (- (`KismetArrayLibrary.Array_Length` (`self.ListBall`)) 1)))
  (bind _returnvalue_2 (`KismetMathLibrary.RandomIntegerInRange` 0 (- (`KismetArrayLibrary.Array_Length` (`self.ListBall`)) 1)))
  (set `self.Ball1` (`|GetArrayItem` (`self.ListBall`) _returnvalue_2))
  (bind _output_get (set `self.Ball2` (`|GetArrayItem` (`self.ListBall`) (`KismetMathLibrary.RandomIntegerInRange` 0 (- (`KismetArrayLibrary.Array_Length` (`self.ListBall`)) 1))) :!label _label))
  (if (`|EnumInequality` (`.TypeName_5_BF24237E4E76D00722C82F9C894F6550` (break `/Game/Data/S_Ball` (`self.Ball1`))) (`.TypeName_5_BF24237E4E76D00722C82F9C894F6550` (break `/Game/Data/S_Ball` _output_get)))
    (bind _output_get_2 (set `self.Ball3` (`|GetArrayItem` (`self.ListBall`) _returnvalue) :!label _label_2))
    (bind _typename (break `/Game/Data/S_Ball` _output_get_2))
    (if (`|EnumInequality` (`.TypeName_5_BF24237E4E76D00722C82F9C894F6550` (break `/Game/Data/S_Ball` (`self.Ball1`))) _typename)
      (if (`|EnumInequality` _typename (`.TypeName_5_BF24237E4E76D00722C82F9C894F6550` (break `/Game/Data/S_Ball` (`self.Ball2`))))
        (`KismetArrayLibrary.Array_Remove` _listball _returnvalue_2)
        (`KismetArrayLibrary.Array_Remove` _listball _returnvalue_2)
        (`KismetArrayLibrary.Array_Remove` _listball _returnvalue)
        (else
          (goto _label_2)))
      (else
        (goto _label_2)))
    (else
      (goto _label))))

(fn `InitBall`
  (bind _outrownames (`DataTableFunctionLibrary.GetDataTableRowNames` "/Game/Data/DB_Ball.DB_Ball"))
  (for _array_element _outrownames
    (bind _returnvalue (`|GetDataTableRow` "/Game/Data/DB_Ball.DB_Ball" _array_element)
      (:`then`
        (switch `/Game/Data/E_Ball` (`.TypeName_5_BF24237E4E76D00722C82F9C894F6550` (break `/Game/Data/S_Ball` _returnvalue))
          (:`NewEnumerator0`
            (set `self.Fire` _returnvalue))
          (:`NewEnumerator1`
            (set `self.Water` _returnvalue))
          (:`NewEnumerator2`
            (set `self.Wood` _returnvalue))
          (:`NewEnumerator3`
            (set `self.Lightning` _returnvalue))
          (:`NewEnumerator4`
            (set `self.Darkness` _returnvalue)))))))

(fn `Set Ball Skill`)