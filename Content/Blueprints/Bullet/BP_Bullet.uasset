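; Team-based bullet projectile that reacts when it hits a character from another team.
; On a sphere collider hit it calls UpdateBall on the opposing BP_CharacterBase and destroys itself, ignoring teammates and other actors.
; The construction script randomizes initial speed up to MaxSpeed, which also caps the projectile movement.
; Activation of the movement component starts a TimeExits delay that destroys the bullet.
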(event `self.SphereCollider.OnComponentHit`
  (params (HitComponent :type "PrimitiveComponent Object Reference") (OtherActor :type "Actor Object Reference") (OtherComp :type "PrimitiveComponent Object Reference") (NormalImpulse :type "Vector Structure") (Hit :type "HitResult Structure (by ref)"))
  (bind _asbp_character_base (cast `/Game/Blueprints/BP_CharacterBase` OtherActor))
  (if (not (`|EnumEquality` (`self.Team`) (`/Game/Blueprints/BP_CharacterBase.Team` _asbp_character_base)))
    (`/Game/Blueprints/BP_CharacterBase.UpdateBall` :`self` _asbp_character_base)
    (`self.K2_DestroyActor`)))

(event `self.ProjectileMovement.OnComponentActivated`
  (params (Component :type "ActorComponent Object Reference") (bReset :type Boolean))
  (`KismetSystemLibrary.Delay` (`self.TimeExits`))
  (`self.K2_DestroyActor`))

(fn `UserConstructionScript`
  (bind _projectilemovement (`self.ProjectileMovement`))
  (set `ProjectileMovementComponent.InitialSpeed` (`KismetMathLibrary.RandomFloatInRange` 1000.0 (`self.Max Speed`)) _projectilemovement)
  (set `ProjectileMovementComponent.MaxSpeed` (`self.Max Speed`) _projectilemovement))