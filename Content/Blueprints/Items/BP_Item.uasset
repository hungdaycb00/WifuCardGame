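; BP_Item is a moving item that holds a random assortment of balls and offers a character-selection widget when bought.
; InterpToMovement carries it along two relative control points set in the construction script.
; On BeginPlay it rolls random DB_Ball rows, tallies quantities by type in the Info map, and feeds them to icons for the controller's first three characters.
; Buy stops movement and reveals the widget.
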(event `self.ReceiveBeginPlay`
  (bind _as_wbp_select_character (`self.As WBP Select Character`))
  (bind _info (`self.Info`))
  (`|ExecutionSequence`
    (:`then_0`
      (bind _aswbp_select_character (cast `/Game/Blueprints/UI/WBP_SelectCharacter` (`WidgetComponent.GetWidget` (`self.Widget`))))
      (set `self.As WBP Select Character` _aswbp_select_character))
    (:`then_1`
      (`self.Init`)
      (`self.CreateItem`))
    (:`then_2`
      (bind _asmy_game_controller (cast `/Game/Blueprints/MyGameController` (`GameplayStatics.GetPlayerController` 0)))
      (for (_array_element _array_index) (`/Game/Blueprints/MyGameController.ListCharacter` _asmy_game_controller)
        (switch `int` _array_index
          (:`0`
            (`/Game/Blueprints/UI/WBP_Icon.SetValue` (`/Game/Blueprints/UI/WBP_SelectCharacter.WBP_Icon` _as_wbp_select_character) _info _array_element self))
          (:`1`
            (`/Game/Blueprints/UI/WBP_Icon.SetValue` (`/Game/Blueprints/UI/WBP_SelectCharacter.WBP_Icon_1` _as_wbp_select_character) _info _array_element self))
          (:`2`
            (`/Game/Blueprints/UI/WBP_Icon.SetValue` (`/Game/Blueprints/UI/WBP_SelectCharacter.WBP_Icon_2` _as_wbp_select_character) _info _array_element self)))))))

(fn `Buy`
  (`MovementComponent.StopMovementImmediately` (`self.InterpToMovement`))
  (`SceneComponent.SetHiddenInGame` (`self.Widget`) false false))

(fn `CreateItem`
  (bind _info (`self.Info`))
  (for _ (range 1 (+ (`self.TotalBall`) 1))
    (bind _out_row (`self.GetRandomBall`))
    (bind _typename (break `/Game/Data/S_Ball` _out_row))
    (if (`BlueprintMapLibrary.Map_Contains` (`self.Info`) _typename)
      (bind _value (`BlueprintMapLibrary.Map_Find` _info _typename))
      (bind (_typename_2 _quantity _icon) (break `/Game/Data/S_Ball` _value))
      (bind _result (`/Engine/EditorBlueprintResources/StandardMacros.IncrementInt` _quantity)
        (:`  `
          (bind _structout (setmembers `/Game/Data/S_Ball` :`StructRef` _value :`TypeName` _typename_2 :`Quantity` _result :`Icon` _icon))
          (`BlueprintMapLibrary.Map_Add` _info _typename_2 _structout)))
      (else
        (`BlueprintMapLibrary.Map_Add` (`self.Info`) _typename _out_row)))))

(fn `GetRandomBall`
  (returns (`Out Row` :type "/Game/Data/S_Ball Structure"))
  (bind _returnvalue (`|GetDataTableRow` "/Game/Data/DB_Ball.DB_Ball" (`KismetStringLibrary.Conv_StringToName` (`|GetEnumeratorNameAsString` (cast `/Game/Data/E_Ball` (`KismetMathLibrary.Conv_IntToByte` (`KismetMathLibrary.RandomIntegerInRange` 0 (- (enumcount `/Game/Data/E_Ball`) 1)))))))
    (:`then`
      (return _returnvalue))))

(fn `Init`
  (`self.TotalBallInit`)
  (`self.GetRandomBall`))

(fn `TotalBallInit`
  (set `self.TotalBall` (`KismetMathLibrary.RandomIntegerInRange` 3 6)))

(fn `UserConstructionScript`
  (bind _interptomovement (`self.InterpToMovement`))
  (set `InterpToMovementComponent.ControlPoints` (`|MakeArray` (make `InterpControlPoint` (`self.Pos1`)) (make `InterpControlPoint` (`self.Pos2`))) _interptomovement)
  (set `InterpToMovementComponent.Duration` 5.0 _interptomovement))